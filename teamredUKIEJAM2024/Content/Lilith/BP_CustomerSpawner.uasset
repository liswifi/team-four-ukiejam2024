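; BP_CustomerSpawner is an actor that spawns BP_Customer actors one at a time from an ordered CustomerList.
; BeginPlay schedules the first SpawnNextCustomer with a short one-shot timer.
; Each call increments CustomerNumber, spawns at the spawner's transform with that list entry as Info, then passes TargetPoint to the customer's Init.
; BeginDay resets the index, and no bounds check guards the list.
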(event `BeginDay`
  (set `self.customerNumber` -1))

(event `self.ReceiveBeginPlay`
  (`KismetSystemLibrary.K2_SetTimerDelegate` (delegate `SpawnNextCustomer`) 2.0))

(event `SpawnNextCustomer`
  (bind _customernumber (`self.customerNumber`))
  (`/Engine/EditorBlueprintResources/StandardMacros.IncrementInt` _customernumber
    (:`  `
      (bind _returnvalue (`|SpawnActorFromClass` "/Game/Lilith/BP_Customer.BP_Customer_C" (`self.GetTransform`) "Undefined" "MultiplyWithRoot" null (`|GetArrayItem` (`self.CustomerList`) _customernumber) null))
      (`/Game/Lilith/BP_Customer.Init` _returnvalue (`self.targetPoint`)))))

(fn `UserConstructionScript`)