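; Cash register prop with Free, Fair and Scam buttons for submitting a decision to a manager, plus a widget money meter showing a settable percentage.
; Interact matches the hit collision to a button while buttons are interactable, then disables them and records the choice.
; A shared timeline animates the pressed button along Y/Z and calls MakeDecision when finished.
; Another timeline fades the buttons' Fresnel colour through dynamic materials to signal availability.
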(event `self.ReceiveBeginPlay`
  (bind (_relativelocation_x _relativelocation_y _relativelocation_z) (`KismetMathLibrary.BreakVector` (`SceneComponent.RelativeLocation` (`self.Button_Free`))))
  ;[1 1 1] Init
  (bind _asw_money_bar (cast `/Game/Lilith/Props/CashRegister/W_MoneyBar` (`WidgetComponent.GetWidget` (`self.moneyMeter`))))
  (set `self.As W Money Bar` _asw_money_bar)
  (set `self.buttonStartY` _relativelocation_y)
  (set `self.buttonStartZ` _relativelocation_z)
  (`self.SetupTextures`))

(event `SetupTextures`
  ;[1 1 1] Init
  (`|ExecutionSequence`
    (:`then_0`
      (bind _returnvalue (`PrimitiveComponent.CreateDynamicMaterialInstance` (`self.Button_Free`) 0 null "None"))
      (bind _output_get (set `self.Mat_Free` _returnvalue))
      (`KismetArrayLibrary.Array_Add` (`self.ButtonMats`) _output_get))
    (:`then_1`
      (bind _returnvalue_2 (`PrimitiveComponent.CreateDynamicMaterialInstance` (`self.Button_Fair`) 0 null "None"))
      (bind _output_get_2 (set `self.Mat_Fair` _returnvalue_2))
      (`KismetArrayLibrary.Array_Add` (`self.ButtonMats`) _output_get_2))
    (:`then_2`
      (bind _returnvalue_3 (`PrimitiveComponent.CreateDynamicMaterialInstance` (`self.Button_Scam`) 0 null "None"))
      (bind _output_get_3 (set `self.Mat_Scam` _returnvalue_3))
      (`KismetArrayLibrary.Array_Add` (`self.ButtonMats`) _output_get_3))))

(event `UpdateMoneyPercent`
  (params (newPercent :type "Float (double-precision)"))
  (set `ProgressBar.Percent` newPercent (`/Game/Lilith/Props/CashRegister/W_MoneyBar.ProgressBar_47` (`self.As W Money Bar`))))

(event `ActivateFresnel`
  ;[1 1 1] Lerps Fresnel Colour rather than boolean-ing
  (set `self.buttonsInteractable?` true)
  (bind (_direction _alpha) (`Timeline|lerpColour` :!label _label)
    (:`Update`
      (for _array_element (`self.ButtonMats`)
        (bind (_returnvalue_x _returnvalue_y _returnvalue_z) (`KismetMathLibrary.BreakVector` (`KismetMathLibrary.VLerp` (0.0 0.0 0.0) (0.0 1.0 1.0) _alpha)))
        (`MaterialInstanceDynamic.SetVectorParameterValue` _array_element "FresnelColour" (`KismetMathLibrary.MakeColor` _returnvalue_x _returnvalue_y _returnvalue_z))))))

(event `DeactivateFresnel`
  ;[1 1 1] Lerps Fresnel Colour rather than boolean-ing
  (set `self.buttonsInteractable?` false)
  (goto _label :!via `Reverse`))

(event `Free_Interact`
  (bind _movingbutton (`self.movingButton`))
  (bind _buttonstarty (`self.buttonStartY`))
  (bind _buttonstartz (`self.buttonStartZ`))
  (bind _relativelocation_x (`KismetMathLibrary.BreakVector` (`SceneComponent.RelativeLocation` _movingbutton)))
  ;[1 1 1] Button Animation
  (set `self.movingButton` (`self.Button_Free`))
  (bind (_direction _newtrack_0) (`Timeline|ButtonMotion` :!via `PlayFromStart` :!label _label_2)
    (:`Update`
      (bind (_returnvalue_x _returnvalue_y _returnvalue_z) (`KismetMathLibrary.BreakVector` (`KismetMathLibrary.VLerp` (`KismetMathLibrary.MakeVector` 0.0 _buttonstarty _buttonstartz) (`KismetMathLibrary.MakeVector` 0.0 (+ _buttonstarty (`self.buttonOffsetY`)) (+ _buttonstartz (`self.buttonOffsetZ`))) _newtrack_0)))
      (`SceneComponent.K2_SetRelativeLocation` _movingbutton (`KismetMathLibrary.MakeVector` _relativelocation_x _returnvalue_y _returnvalue_z) false false))
    (:`Finished`
      (`/Game/Lilith/Customers/BP_CustomerManager.MakeDecision` (`self.manager`) (`self.currentDecision`)))))

(event `Fair_Interact`
  ;[1 1 1] Button Animation
  (set `self.movingButton` (`self.Button_Fair`))
  (goto _label_2 :!via `PlayFromStart`))

(event `Scam_Interact`
  ;[1 1 1] Button Animation
  (set `self.movingButton` (`self.Button_Scam`))
  (goto _label_2 :!via `PlayFromStart`))

(event `/Game/Tori/I_Interact.Interact`
  (params (IsClicking :type Boolean) (playerRef :type "/Game/Tori/BP_PlayerTori Object Reference") (hitComponent :type "ActorComponent Object Reference"))
  ;[1 1 1] Button Interact
  (if (`self.buttonsInteractable?`)
    (bind _output_get (set `self.HitComponent` hitComponent))
    ;;[1 1 1] Free Button?
    (if (== _output_get (`self.Coll_Free`))
      (`self.Free_Interact`)
      (`self.DeactivateFresnel`)
      (set `self.currentDecision` "NewEnumerator1")
      (else
        ;;[1 1 1] Fair Button?
        (if (== (`self.HitComponent`) (`self.Coll_Fair`))
          (`self.Fair_Interact`)
          (`self.DeactivateFresnel`)
          (set `self.currentDecision` "NewEnumerator2")
          (else
            ;;[1 1 1] Scam Button?
            (if (== (`self.HitComponent`) (`self.Coll_Scam`))
              (`self.Scam_Interact`)
              (`self.DeactivateFresnel`)
              (set `self.currentDecision` "NewEnumerator3"))))))))

(fn `GetPercentage`
  (returns (Percent :type "Float (double-precision)"))
  (return (`ProgressBar.Percent` (`/Game/Lilith/Props/CashRegister/W_MoneyBar.ProgressBar_47` (`self.As W Money Bar`)))))

(fn `UserConstructionScript`)