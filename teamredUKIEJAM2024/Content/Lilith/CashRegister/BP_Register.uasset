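; Cash register actor with Free, Fair and Scam buttons that animate when their interact events run.
; Each event sets the moving button and restarts one shared timeline, which offsets it in local Y and Z from ButtonFree's starting position.
; BeginPlay caches that position and fires the three events on staggered one-shot timers.
; The timeline's finish calls StartDialogue, which is an empty stub.
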(event `self.ReceiveBeginPlay`
  (bind (_relativelocation_x _relativelocation_y _relativelocation_z) (`KismetMathLibrary.BreakVector` (`SceneComponent.RelativeLocation` (`self.Button_Free`))))
  (set `self.buttonStartY` _relativelocation_y)
  (set `self.buttonStartZ` _relativelocation_z)
  (`KismetSystemLibrary.K2_SetTimerDelegate` (delegate `Free_Interact`) 1.5)
  (`KismetSystemLibrary.K2_SetTimerDelegate` (delegate `Fair_Interact`) 3.0)
  (`KismetSystemLibrary.K2_SetTimerDelegate` (delegate `Scam_Interact`) 4.5))

(event `Free_Interact`
  (bind _movingbutton (`self.movingButton`))
  (bind _buttonstarty (`self.buttonStartY`))
  (bind _buttonstartz (`self.buttonStartZ`))
  (bind _relativelocation_x (`KismetMathLibrary.BreakVector` (`SceneComponent.RelativeLocation` _movingbutton)))
  (set `self.movingButton` (`self.Button_Free`))
  (bind (_direction _newtrack_0) (`Timeline|ButtonMotion` :!via `PlayFromStart` :!label _label)
    (:`Update`
      (bind (_returnvalue_x _returnvalue_y _returnvalue_z) (`KismetMathLibrary.BreakVector` (`KismetMathLibrary.VLerp` (`KismetMathLibrary.MakeVector` 0.0 _buttonstarty _buttonstartz) (`KismetMathLibrary.MakeVector` 0.0 (+ _buttonstarty (`self.buttonOffsetY`)) (+ _buttonstartz (`self.buttonOffsetZ`))) _newtrack_0)))
      (`SceneComponent.K2_SetRelativeLocation` _movingbutton (`KismetMathLibrary.MakeVector` _relativelocation_x _returnvalue_y _returnvalue_z) false false))
    (:`Finished`
      (`self.Start Dialogue`))))

(event `Fair_Interact`
  (set `self.movingButton` (`self.Button_Fair`))
  (goto _label :!via `PlayFromStart`))

(event `Scam_Interact`
  (set `self.movingButton` (`self.Button_Scam`))
  (goto _label :!via `PlayFromStart`))

(event `Start Dialogue`)

(fn `UserConstructionScript`)