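; BP_Customer is a shop customer that travels to a window, holds a dialogue, then leaves and has its manager spawn the next customer.
; Horizontal and vertical timelines drive movement with a height offset, reversing the horizontal one to exit, while rotation timelines turn it at each end.
; On arrival it shows its Info dialogue and activates the register's fresnel.
; Respond picks a reply and mood material from the Free, Fair or Scam decision.
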(event `Init`
  (params (MoveTarget :type "/Game/Lilith/BP_VectorPoint Object Reference"))
  (bind (_returnvalue_x _returnvalue_y _returnvalue_z) (`KismetMathLibrary.BreakVector` (`self.K2_GetActorLocation`)))
  (bind (_returnvalue_x_2 _returnvalue_y_2) (`KismetMathLibrary.BreakVector` (`self.K2_GetActorLocation` (`self.targetPoint`))))
  (`SkeletalMeshComponent.SetSkeletalMeshAsset` (`self.SkeletalMesh`) (`.Mesh_44_C2A84B124CDAAAA2D297329CBCD65016` (break `/Game/Lilith/Customers/S_Customer` (`self.Info`))))
  (set `self.targetPoint` MoveTarget)
  (set `self.startHeight` _returnvalue_z)
  (set `self.startHorizontal` _returnvalue_y)
  (set `self.endHorizontal` _returnvalue_y_2)
  (`self.Move To Window`))

(event `LeaveWindow`
  (bind _returnvalue_x (`KismetMathLibrary.BreakVector` (`self.K2_GetActorLocation`)))
  (bind _startheight (`self.startHeight`))
  (set `self.leaving?` true)
  (bind (_direction _rotation) (`Timeline|Rotation_leaving`)
    (:`Update`
      (`self.K2_SetActorRotation` (`KismetMathLibrary.RLerp` (struct :`Yaw` -90.0) (struct :`Yaw` -180.0) _rotation)))
    (:`Finished`
      (`|ExecutionSequence`
        (:`then_0`
          ;[1 1 1] Customer animation
          (bind (_direction_2 _horizontal) (`Timeline|Motion_H` :!via `Reverse` :!label _label)
            (:`Update`
              (`self.K2_SetActorLocation` (`KismetMathLibrary.MakeVector` _returnvalue_x (`KismetMathLibrary.Lerp` (`self.startHorizontal`) (`self.endHorizontal`) _horizontal) (`KismetMathLibrary.Lerp` _startheight (+ _startheight (`self.HeightOffset`)) (stale _newtrack_0)))))
            (:`Finished`
              (`self.EndMove`))))
        (:`then_1`
          (bind (_direction_3 _newtrack_0) (`Timeline|Motion_V` :!label _label_2)))))))

(event `Move To Window`
  ;[1 1 1] Customer animation
  (`|ExecutionSequence`
    (:`then_0`
      (goto _label))
    (:`then_1`
      (goto _label_2))))

(event `EndMove`
  ;[1 1 1] Customer animation
  (`|ExecutionSequence`
    (:`then_0`
      (goto _label_2 :!via `Stop`))
    (:`then_1`
      (if (`self.leaving?`)
        (`/Game/Lilith/Customers/BP_CustomerManager.SpawnNextCustomer` (`self.Manager`))
        (else
          (bind (_direction _rotation) (`Timeline|Rotation`)
            (:`Update`
              (`self.K2_SetActorRotation` (`KismetMathLibrary.RLerp` (struct) (struct :`Yaw` -90.0) _rotation)))
            (:`Finished`
              ;[1 1 1] Start Dialogue
              (`/Game/Tori/Dialogue/W_Dialogue.InsertNewDialogue` (`self.Dialogue HUD`) (`.Dialogue_34_7FEF8F13467E84097EED16B1BB513359` (break `/Game/Lilith/Customers/S_Customer` (`self.Info`))))
              (`/Game/Lilith/Props/CashRegister/BP_Register.ActivateFresnel` (`self.Register`)))))))))

(event `Respond`
  (params (Decision :type "/Game/Lilith/E_Outcome Enum" :default "NewEnumerator0"))
  (bind (_dialogue _positiveresponse _nuetralresponse _negativeresponse) (break `/Game/Lilith/Customers/S_Customer` (`self.Info`)))
  (`/Game/Tori/Dialogue/W_Dialogue.InsertNewDialogue` (`self.Dialogue HUD`) (select `/Game/Lilith/E_Outcome` Decision :`NewEnumerator1` _positiveresponse :`NewEnumerator2` _nuetralresponse :`NewEnumerator3` _negativeresponse))
  (`PrimitiveComponent.SetMaterial` (`self.SkeletalMesh`) 0 (select `/Game/Lilith/E_Outcome` Decision :`NewEnumerator1` "/Game/Lilith/Customers/FaceMats/M_Happy.M_Happy" :`NewEnumerator2` "/Game/Lilith/Customers/FaceMats/M_Nuetral.M_Nuetral" :`NewEnumerator3` "/Game/Lilith/Customers/FaceMats/M_Angry.M_Angry" :!type "MaterialInterface Object Reference")))

(fn `UserConstructionScript`)