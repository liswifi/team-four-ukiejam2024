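; Customer manager that runs a shop day, spawning customers from a list one at a time and tracking the player's Money and Integrity.
; BeginDay starts spawning after a short delay, and each customer receives the dialogue HUD, register and manager references.
; Free, Fair or Scam decisions go to the active customer and adjust both clamped stats; InvestigatorScam also cuts Integrity.
; An exhausted list fades the screen out, while EndDayEarly (on zero Money) and IntegrityCheck are empty stubs.
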(event `IntegrityCheck`)

(event `EndDayEarly`)

(event `Init`
  (params (HUD :type "/Game/Tori/UI/W_HUD Object Reference"))
  (set `self.HUD` HUD))

(event `BeginDay`
  (set `self.customerNumber` -1)
  (`KismetSystemLibrary.K2_SetTimerDelegate` (delegate `SpawnNextCustomer`) 2.0))

(event `SpawnNextCustomer`
  (bind _customernumber (`self.customerNumber`))
  (if (<= (`self.Money`) 0.0)
    (`self.EndDayEarly`)
    (else
      (`/Engine/EditorBlueprintResources/StandardMacros.IncrementInt` _customernumber
        (:`  `
          (if (== (`KismetArrayLibrary.Array_Length` (`self.CustomerList`)) (`self.customerNumber`))
            (`PlayerCameraManager.StartCameraFade` :`self` (`GameplayStatics.GetPlayerCameraManager` 0) :`ToAlpha` 1.0 :`Duration` 3.0 :`bHoldWhenFinished` true)
            (else
              (bind _returnvalue (`|SpawnActorFromClass` "/Game/Lilith/Customers/BP_Customer.BP_Customer_C" (`self.GetTransform`) "Undefined" "MultiplyWithRoot" null (`|GetArrayItem` (`self.CustomerList`) _customernumber) (`/Game/Tori/UI/W_HUD.W_Dialogue` (`self.HUD`)) (`self.Register`) self null))
              (`/Game/Lilith/Customers/BP_Customer.Init` _returnvalue (`self.targetPoint`))
              (set `self.activeCustomer` _returnvalue))))))))

(event `MakeDecision`
  (params (Decision :type "/Game/Lilith/E_Outcome Enum" :default "NewEnumerator0"))
  (set `self.CustomerResponding?` true)
  (`/Game/Lilith/Customers/BP_Customer.Respond` (`self.activeCustomer`) Decision)
  (switch `/Game/Lilith/E_Outcome` Decision
    (:`NewEnumerator1`
      ;[1 1 1] Free Outcome
      (set `self.Money` (`KismetMathLibrary.FClamp` (+ (`self.Money`) -10.0) 0.0 100.0))
      (set `self.Integrity` (`KismetMathLibrary.FClamp` (+ (`self.Integrity`) 20.0) 0.0 100.0)))
    (:`NewEnumerator2`
      ;[1 1 1] Fair Outcome
      (set `self.Money` (`KismetMathLibrary.FClamp` (+ (`self.Money`) 0.0) 0.0 100.0))
      (set `self.Integrity` (`KismetMathLibrary.FClamp` (+ (`self.Integrity`) -5.0) 0.0 100.0)))
    (:`NewEnumerator3`
      ;[1 1 1] Scam Outcome
      (set `self.Money` (`KismetMathLibrary.FClamp` (+ (`self.Money`) 10.0) 0.0 100.0))
      (set `self.Integrity` (`KismetMathLibrary.FClamp` (+ (`self.Integrity`) -15.0) 0.0 100.0))))
  (`KismetSystemLibrary.PrintString` (`KismetStringLibrary.Concat_StrStr` "Money=" (`KismetStringLibrary.Conv_DoubleToString` (`self.Money`)) " / " "Integrity=" (`KismetStringLibrary.Conv_DoubleToString` (`self.Integrity`)))))

(event `CustomerLeavesIfResponse`
  (if (`self.CustomerResponding?`)
    (`/Game/Lilith/Customers/BP_Customer.LeaveWindow` (`self.activeCustomer`))
    (set `self.CustomerResponding?` false)))

(event `InvestigatorScam`
  (set `self.Integrity` (`KismetMathLibrary.FClamp` (+ (`self.Integrity`) -15.0) 0.0 100.0))
  (`KismetSystemLibrary.PrintString` (`KismetStringLibrary.Concat_StrStr` "Money=" (`KismetStringLibrary.Conv_DoubleToString` (`self.Money`)) " / " "Integrity=" (`KismetStringLibrary.Conv_DoubleToString` (`self.Integrity`)))))

(fn `UserConstructionScript`)