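; BP_Customer is a customer actor that travels along the Y axis to a target point, apparently a window, with a vertical offset motion.
; Init stores the target, calls mesh and material setters, caches start and end coordinates, then starts the move.
; Two timelines run together: Motion_H's update lerps Y and applies Motion_V's curve to Z, scaled by HeightOffset.
; When Motion_H finishes, EndMove stops Motion_V.
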(event `Init`
  (params (MoveTarget :type "/Game/Lilith/BP_VectorPoint Object Reference"))
  (bind (_returnvalue_x _returnvalue_y _returnvalue_z) (`KismetMathLibrary.BreakVector` (`self.K2_GetActorLocation`)))
  (bind _mesh (`self.Mesh`))
  (bind (_returnvalue_x_2 _returnvalue_y_2) (`KismetMathLibrary.BreakVector` (`self.K2_GetActorLocation` (`self.targetPoint`))))
  (set `self.targetPoint` MoveTarget)
  (`StaticMeshComponent.SetStaticMesh` _mesh null)
  (`PrimitiveComponent.SetMaterial` _mesh 0 null)
  (set `self.startHeight` _returnvalue_z)
  (set `self.startHorizontal` _returnvalue_y)
  (set `self.endHorizontal` _returnvalue_y_2)
  (`self.Move To Window`))

(event `Move To Window`
  (bind _returnvalue_x (`KismetMathLibrary.BreakVector` (`self.K2_GetActorLocation`)))
  (bind _startheight (`self.startHeight`))
  (`|ExecutionSequence`
    (:`then_0`
      (bind (_direction _horizontal) (`Timeline|Motion_H`)
        (:`Update`
          (`self.K2_SetActorLocation` (`KismetMathLibrary.MakeVector` _returnvalue_x (`KismetMathLibrary.Lerp` (`self.startHorizontal`) (`self.endHorizontal`) _horizontal) (`KismetMathLibrary.Lerp` _startheight (+ _startheight (`self.HeightOffset`)) (stale _newtrack_0)))))
        (:`Finished`
          (`self.EndMove`))))
    (:`then_1`
      (bind (_direction_2 _newtrack_0) (`Timeline|Motion_V` :!label _label)))))

(event `EndMove`
  (goto _label :!via `Stop`))

(fn `UserConstructionScript`)